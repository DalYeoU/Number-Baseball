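; BP_FoxPlayerController is the player controller that drives the chat UI and game-result popup in a game with a correct answer and winner.
; BeginPlay creates the chat window, received messages append chat item widgets to its scroll log, and Enter focuses the input box.
; Game results show a Korean win or draw message with the answer in a widget removed after a short delay.
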(event `self.OnShowGameResult`
  (params (WinnerName :type String) (bIsDraw :type Boolean) (CorrectAnswer :type String))
  (bind _result (`|FormatText` "정답은 {Answer} 이었습니다." CorrectAnswer))
  (bind _returnvalue (`|CreateWidget` "/Game/Chat/BluePrint/WBP_FoxGameResult.WBP_FoxGameResult_C"))
  (if bIsDraw
    (`/Game/Chat/BluePrint/WBP_FoxGameResult.SetResultMessage` _returnvalue "게임 오버 (무승부!)" _result)
    (`UserWidget.AddToViewport` _returnvalue 0)
    (`KismetSystemLibrary.Delay` 4.0)
    (`Widget.RemoveFromParent` _returnvalue)
    (else
      (`/Game/Chat/BluePrint/WBP_FoxGameResult.SetResultMessage` _returnvalue (`|FormatText` "우승자: {Name}!" WinnerName) _result)
      (`UserWidget.AddToViewport` _returnvalue 0)
      (`KismetSystemLibrary.Delay` 4.0)
      (`Widget.RemoveFromParent` _returnvalue))))

(event `self.ReceiveBeginPlay`
  (bind _returnvalue (`|CreateWidget` "/Game/Chat/BluePrint/WBP_ChatWindow.WBP_ChatWindow_C"))
  (set `self.ChatWindowRef` _returnvalue)
  (`UserWidget.AddToViewport` _returnvalue 0))

(event `self.OnReceiveChatMessage`
  (params (SenderName :type String) (Message :type String))
  (bind _returnvalue (`|CreateWidget` "/Game/Chat/BluePrint/WBP_ChatItem.WBP_ChatItem_C"))
  (`TextBlock.SetText` (`/Game/Chat/BluePrint/WBP_ChatItem.TXT_Name` _returnvalue) (`KismetTextLibrary.Conv_StringToText` SenderName))
  (`TextBlock.SetText` (`/Game/Chat/BluePrint/WBP_ChatItem.TXT_Message` _returnvalue) (`KismetTextLibrary.Conv_StringToText` Message))
  (`PanelWidget.AddChild` (`/Game/Chat/BluePrint/WBP_ChatWindow.Scroll_ChatLog` (`self.ChatWindowRef`)) _returnvalue))

(event `Key|Enter`
  (params (Key :type "Key Structure"))
  (bind _etb_chatinput (`/Game/Chat/BluePrint/WBP_ChatWindow.ETB_ChatInput` (`self.ChatWindowRef`)))
  (:`Pressed`
    (`Widget.SetUserFocus` _etb_chatinput self)
    (`WidgetBlueprintLibrary.SetInputMode_GameAndUIEx` self _etb_chatinput)))

(fn `UserConstructionScript`)